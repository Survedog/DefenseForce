(event EventOnEnterBuildMode
  (params (InTargetStructureClass :type DF%20Structure%20Base%20Class%20Reference))
  (bind _asbp_dfplayer_pawn (Utilities|Casting|CastToBP_DFPlayerPawn (Variables|Default|GetDFPlayerPawn)))
  (Default|OnEnterBuildMode _asbp_dfplayer_pawn InTargetStructureClass))

(event EventBeginPlay
  (|CallParentFunction)
  (if (Pawn|IsLocalController)
    (bind _returnvalue (UserInterface|CreateWidget "/Game/DefenseForce/Blueprint/UI/WBP_HUD.WBP_HUD_C" self))
    (bind _output_get (Variables|Default|SetHUDWidget _returnvalue))
    (Utilities|IsValid _output_get
      (:Is%20Valid
        (UserInterface|Viewport|AddtoViewport _output_get 0)))))

(event EventOnExitBuildMode
  (params (InBuiltStructure :type DF%20Structure%20Base%20Object%20Reference))
  (bind _asbp_dfplayer_pawn (Utilities|Casting|CastToBP_DFPlayerPawn (Variables|Default|GetDFPlayerPawn)))
  (Default|OnExitBuildMode _asbp_dfplayer_pawn InBuiltStructure))

(fn ConstructionScript)