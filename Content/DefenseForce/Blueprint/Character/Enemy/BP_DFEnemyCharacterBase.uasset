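; Base Blueprint for Defense Force enemy characters, handling damage, death and the money reward for a kill.
; AnyDamage subtracts incoming damage from HP through the HP getter and setter.
; OnDead runs the parent logic, then on authority only awards the drop amount through BP_DFGameState and destroys the actor.
; GetDamageAmount supplies a fixed damage value.
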(event EventOnDead
  (|CallParentFunction)
  (Networking|SwitchHasAuthority
    (:Authority
      (bind _asbp_dfgame_state (Utilities|Casting|CastToBP_DFGameState (Game|GetGameState)))
      (Class|DFGameState|EarnMoney _asbp_dfgame_state (Variables|Default|GetDropMoneyAmount))
      (Actor|DestroyActor))))

(event Game|Damage|EventAnyDamage
  (params (Damage :type Float%20%28single-precision%29) (DamageType :type Damage%20Type%20Object%20Reference) (InstigatedBy :type Controller%20Object%20Reference) (DamageCauser :type Actor%20Object%20Reference))
  (Class|DFEnemyCharacter|SetHp (- (Class|DFEnemyCharacter|GetHp) Damage)))

(fn ConstructionScript)

(fn GetDamageAmount
  (return 2e+01))