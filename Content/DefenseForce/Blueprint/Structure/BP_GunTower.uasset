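; Controllable gun tower structure that a player operates to shoot projectiles.
; While controlled, Tick rotates the whole actor in yaw toward the controlling pawn's aim location, keeping the Head component's roll and pitch.
; On control start the server grants a shoot-projectile Gameplay Ability to the player pawn's Ability System Component on an input ID, and clears it by stored handle when control ends.
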(event EventOnControlStart
  (params (NewPlayerPawn :type DF%20Player%20Pawn%20Object%20Reference))
  (bind _returnvalue (Ability|GetAbilitySystemComponent NewPlayerPawn))
  ;[1 1 1] Grant/Remove attack GA to player
  (|CallParentFunction NewPlayerPawn)
  (Networking|SwitchHasAuthority
    (:Authority
      (Utilities|IsValid _returnvalue
        (:Is%20Valid
          (bind _returnvalue_2 (GameplayAbilities|GiveAbility _returnvalue "/Game/DefenseForce/Blueprint/GAS/GA/Tower/BPGA_GunTower_ShootProjectile.BPGA_GunTower_ShootProjectile_C" 0 2))
          (Variables|GAS|SetShoortProjectileAbilityHandle _returnvalue_2))))))

(event EventTick
  (params (DeltaSeconds :type Float%20%28single-precision%29))
  (bind _head (Variables|Default|GetHead))
  (bind _returnvalue (Transformation|GetWorldRotation _head))
  ;[1 1 1] Rotate head to player aim location
  (|CallParentFunction DeltaSeconds)
  (if (Class|DFTowerBase|IsBeingControlled)
    (Transformation|SetActorRotation (Math|Rotator|MakeRotator (.roll _returnvalue) (.pitch _returnvalue) (.yaw (Math|Rotator|FindLookatRotation (Transformation|GetWorldLocation _head) (Variables|/Script/DefenseForce.DFPlayerPawn|GetPlayerAimLocation (Variables|Default|GetControllingPlayerPawn))))))))

(event EventOnControlEnd
  (bind _controllingplayerpawn (Variables|Default|GetControllingPlayerPawn))
  (bind _returnvalue (Ability|GetAbilitySystemComponent _controllingplayerpawn))
  ;[1 1 1] Grant/Remove attack GA to player
  (|CallParentFunction)
  (Networking|SwitchHasAuthority
    (:Authority
      (Utilities|IsValid _returnvalue
        (:Is%20Valid
          (GameplayAbilities|ClearAbility _returnvalue (Variables|GAS|GetShoortProjectileAbilityHandle))
          (Variables|GAS|SetShoortProjectileAbilityHandle ""))))))

(fn ConstructionScript)