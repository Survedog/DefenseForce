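; BP_TowerBase is a base tower Blueprint that tracks where the player aims with the mouse in the world.
; It caches the first PlayerController on BeginPlay and updates PlayerAimLocation every Tick.
; The update deprojects the cursor into a world direction and line-traces on Visibility from the camera location.
; The aim location is the hit point, or the trace's far end at PlayerAimTraceLength when nothing is hit.
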(event Custom|UpdatePlayerAimLocation
  (bind _playercontroller (Variables|Default|GetPlayerController))
  (bind _playeraimtracelength (Variables|Default|GetPlayerAimTraceLength))
  (bind (_locationx _locationy) (Game|Player|GetMousePosition _playercontroller))
  (bind _playercameramanager (Variables|/Script/Engine.PlayerController|GetPlayerCameraManager _playercontroller))
  (bind _returnvalue (Camera|GetCameraLocation _playercameramanager))
  (bind _worlddirection (Class|PlayerController|DeprojectScreenPositiontoWorld _playercontroller _locationx _locationy))
  (bind _returnvalue_2 (* _worlddirection _playeraimtracelength))
  (bind _returnvalue_3 (+ _returnvalue _returnvalue_2))
  (if (Utilities|IsValid (Variables|Default|GetPlayerController))
    (bind (_outhit _returnvalue_4) (Collision|LineTraceByChannel _returnvalue _returnvalue_3 "TraceTypeQuery1" false 0 "None" true "(R=1.000000,G=0.000000,B=0.000000,A=1.000000)" "(R=0.000000,G=1.000000,B=0.000000,A=1.000000)" 1.0))
    (if _returnvalue_4
      (Variables|Default|SetPlayerAimLocation (.Location (Collision|BreakHitResult _outhit)))
      (else
        (Variables|Default|SetPlayerAimLocation _returnvalue_3)))))

(event EventBeginPlay
  (Variables|Default|SetPlayerController (Game|GetPlayerController 0)))

(event EventTick
  (params (DeltaSeconds :type Float%20%28single-precision%29))
  (CallFunction|UpdatePlayerAimLocation))

(fn ConstructionScript)