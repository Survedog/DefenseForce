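; BP_DFTowerBase is a base tower structure Blueprint that lends an attack ability to the player controlling it.
; On control start it calls the parent, then on authority grants AttackAbilityClass to the pawn's Ability System Component and stores the spec handle.
; On control end authority clears that ability and handle before calling the parent, while remotes call the parent directly.
; The authority's parent end call only runs when the component is valid.
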(event EventOnControlStart
  (params (NewPlayerPawn :type DF%20Player%20Pawn%20Object%20Reference))
  (bind _returnvalue (Ability|GetAbilitySystemComponent NewPlayerPawn))
  ;[1 1 1] Grant/Remove attack GA to player
  (|CallParentFunction NewPlayerPawn)
  (Networking|SwitchHasAuthority
    (:Authority
      (Utilities|IsValid _returnvalue
        (:Is%20Valid
          (bind _returnvalue_2 (GameplayAbilities|GiveAbility _returnvalue (Variables|GAS|GetAttackAbilityClass) 0 2))
          (Variables|GAS|SetAttackAbilitySpecHandle _returnvalue_2))))))

(event EventOnControlEnd
  (bind _controllingplayerpawn (Variables|Default|GetControllingPlayerPawn))
  (bind _returnvalue (Ability|GetAbilitySystemComponent _controllingplayerpawn))
  ;[1 1 1] Grant/Remove attack GA to player
  (Networking|SwitchHasAuthority
    (:Authority
      (Utilities|IsValid _returnvalue
        (:Is%20Valid
          (GameplayAbilities|ClearAbility _returnvalue (Variables|GAS|GetAttackAbilitySpecHandle))
          (Variables|GAS|SetAttackAbilitySpecHandle ""))))
    (:Remote
      _))
  (|CallParentFunction))

(fn ConstructionScript)