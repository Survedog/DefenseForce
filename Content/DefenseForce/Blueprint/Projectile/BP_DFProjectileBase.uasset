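; Base projectile for the DefenseForce game that damages enemy characters on contact.
; On actor overlap it applies damage from GetDamageAmount, a fixed default value, only if the other actor is a BP_DFEnemyCharacterBase.
; Any overlap then spawns a pooled Niagara energy-burst effect and destroys the projectile.
; The construction script gives the mesh a dynamic emissive material with a bright blue color.
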(event Collision|EventActorBeginOverlap
  (params (OtherActor :type Actor%20Object%20Reference))
  (bind _asbp_dfenemy_character_base (Utilities|Casting|CastToBP_DFEnemyCharacterBase OtherActor)
    (:then
      (Game|Damage|ApplyDamage _asbp_dfenemy_character_base (CallFunction|GetDamageAmount) (Game|GetInstigatorController) self))
    (:CastFailed
      _))
  (Niagara|SpawnSystematLocation "/Game/DefenseForce/Blueprint/FX/NS_EnergyBulletBurst.NS_EnergyBulletBurst" (Transformation|GetActorLocation) "0, 0, 0" "1.000000,1.000000,1.000000" true true "AutoRelease")
  (Actor|DestroyActor))

(fn ConstructionScript
  (bind _returnvalue (Rendering|Material|CreateDynamicMaterialInstance (Variables|Default|GetStaticMesh) 0 "/Engine/ArtTools/RenderToTexture/Materials/Debug/M_Emissive_Color.M_Emissive_Color" "None" :!class /Script/Engine.PrimitiveComponent))
  (Rendering|Material|SetVectorParameterValue _returnvalue "Color" "(R=0.000000,G=0.000000,B=255.000000,A=1.000000)" :!class /Script/Engine.MaterialInstanceDynamic))

(fn GetDamageAmount
  (return 1e+01))