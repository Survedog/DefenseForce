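; A GAS world reticle that draws a predicted projectile arc and marks its landing point during targeting.
; Each new predict-path result rebuilds a spline from the path's world locations.
; Spline mesh components are added or destroyed to match the segment count, then each spans two neighbouring points.
; The landing indicator moves to the impact point only on a blocking hit.
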(event EventOnTraceResultSet
  (params (HitResult :type Hit%20Result%20Structure%20%28by%20ref%29)))

(event EventOnPredictPathResultSet
  (params (PredictPathResult :type Predict%20Projectile%20Path%20Result%20Structure%20%28by%20ref%29))
  (bind (_pathdata _lasttracedestination _hitresult) (Utilities|Struct|BreakPredictProjectilePathResult PredictPathResult))
  (bind _spline (Variables|Default|GetSpline))
  (bind _splinemesharray (Variables|Default|GetSplineMeshArray))
  (bind _splinemesharray_2 (Variables|Default|GetSplineMeshArray))
  (bind _spline_2 (Variables|Default|GetSpline))
  (bind _splinemesharray_3 (Variables|Default|GetSplineMeshArray))
  (bind _returnvalue (Utilities|Array|Length _splinemesharray_2))
  (bind _returnvalue_2 (Utilities|Array|Length _splinemesharray_3))
  (bind (_bblockinghit _binitialoverlap _time _distance _location _impactpoint) (Collision|BreakHitResult _hitresult))
  (bind _returnvalue_3 (Spline|GetNumberOfSplinePoints _spline_2))
  (bind _returnvalue_4 (Utilities|Operators|Subtract _returnvalue_3 _returnvalue_2 1))
  (bind _returnvalue_5 (+ _returnvalue_4 _returnvalue))
  (Utilities|FlowControl|Sequence
    (:then_0
      ;[1 1 1] Add Projectile Path Points To Spline
      (Spline|ClearSplinePoints (Variables|Default|GetSpline) true)
      (for _array_element _pathdata
        (Spline|AddSplinePoint (Variables|Default|GetSpline) (.Location (Utilities|Struct|BreakPredictProjectilePathPointData _array_element)) "World" true)))
    (:then_1
      ;[1 1 1] Adjust The Number of Spline Mesh Components
      (if (> _returnvalue_4 0)
        (for _index (range 0 _returnvalue_4)
          (bind _returnvalue_6 (AddComponent|AddSplineMeshComponent false))
          (Utilities|Array|Add (Variables|Default|GetSplineMeshArray) _returnvalue_6))
        (elif (< _returnvalue_4 0)
          (for _index_2 (range _returnvalue_5 (- _returnvalue 1))
            (Components|DestroyComponent (Utilities|Array|Get(acopy) _splinemesharray _index_2)))
          (Utilities|Array|Resize _splinemesharray _returnvalue_5))))
    (:then_2
      ;[1 1 1] Set Start And End Position of Each Spline Mesh
      (for _index_3 (range 0 (- _returnvalue_2 1))
        (SplineMesh|SetStartandEnd (Utilities|Array|Get(acopy) (Variables|Default|GetSplineMeshArray) _index_3) (Spline|GetLocationatSplinePoint _spline _index_3 "World") "0, 0, 0" (Spline|GetLocationatSplinePoint _spline (+ _index_3 1) "World") "0, 0, 0" true :!class /Script/Engine.SplineMeshComponent)))
    (:then_3
      ;[1 1 1] Locate Landing Point Indicator
      (if _bblockinghit
        (Transformation|SetWorldLocation (Variables|Default|GetLandingPointIndicator) _impactpoint false true)))))

(fn ConstructionScript)