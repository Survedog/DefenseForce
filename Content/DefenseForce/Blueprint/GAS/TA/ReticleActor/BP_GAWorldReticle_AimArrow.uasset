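; Gameplay Ability world reticle that draws a ground-level arrow from a tower toward the targeted point.
; On parameter initialization it snaps to the XY position of its owner's owner, the tower, at a fixed height just above zero.
; Each trace result sets the spline mesh's end to the horizontal distance to the hit and yaws the actor to face it, so the arrow stretches and turns flat.
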(event EventOnParametersInitialized
  (bind _returnvalue (Components|GetOwner))
  (bind _returnvalue_2 (Components|GetOwner _returnvalue))
  (bind _returnvalue_3 (Transformation|GetActorLocation _returnvalue_2))
  (Transformation|SetActorLocation (Math|Vector|MakeVector (.x _returnvalue_3) (.y _returnvalue_3) 1.0) false false))

(event EventOnTraceResultSet
  (params (HitResult :type Hit%20Result%20Structure%20%28by%20ref%29))
  (bind _returnvalue (Transformation|GetActorLocation))
  (bind _location (Collision|BreakHitResult HitResult))
  (bind _returnvalue_2 (- _location _returnvalue))
  (SplineMesh|SetEndPosition (Variables|Default|GetSplineMesh) (Math|Vector|MakeVector (Math|Vector2D|Vector2DLength (Math|Conversions|ToVector2D(Vector) _returnvalue_2)) 0.0 0.0) true)
  (Transformation|SetActorRotation (Math|Rotator|MakeRotator 0.0 0.0 (.yaw (Math|Rotator|MakeRotfromX _returnvalue_2)))))

(fn ConstructionScript)