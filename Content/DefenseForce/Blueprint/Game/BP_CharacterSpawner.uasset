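; BP_CharacterSpawner is a server-authoritative actor that repeatedly spawns characters of a configurable class around its own location.
; On BeginPlay, StartSpawning runs on authority and starts a looping timer at the spawn cooldown.
; Each tick of the timer spawns the class at the spawner's transform plus a random per-axis offset, using a configurable collision handling method.
; EndSpawning clears the stored timer handle to stop spawning.
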(event Custom|SpawnCharacter
  (bind _returnvalue (Transformation|GetActorTransform))
  (bind _minrandomspawnoffset (Variables|Spawner|GetMinRandomSpawnOffset))
  (bind _maxrandomspawnoffset (Variables|Spawner|GetMaxRandomSpawnOffset))
  (Networking|SwitchHasAuthority
    (:Authority
      (Game|SpawnActorfromClass (Variables|Spawner|GetSpawnedCharacterClass) (Math|Transform|MakeTransform (+ (Math|Vector|MakeVector (Math|Random|RandomFloatinRange (.x _minrandomspawnoffset) (.x _maxrandomspawnoffset)) (Math|Random|RandomFloatinRange (.y _minrandomspawnoffset) (.y _maxrandomspawnoffset)) (Math|Random|RandomFloatinRange (.z _minrandomspawnoffset) (.z _maxrandomspawnoffset))) (.location _returnvalue)) (.rotation _returnvalue) (.scale _returnvalue)) (Variables|Spawner|GetSpawnCollisionMethod) "MultiplyWithRoot" 0 0))))

(event Custom|EndSpawning
  (bind _spawntimerhandle (Variables|Spawner|GetSpawnTimerHandle))
  (if (Utilities|Time|IsValidTimerHandle _spawntimerhandle)
    (Utilities|Time|ClearandInvalidateTimerbyHandle _spawntimerhandle)))

(event Custom|StartSpawning
  (Networking|SwitchHasAuthority
    (:Authority
      (bind _returnvalue (Utilities|Time|SetTimerbyEvent (delegate Custom|SpawnCharacter) (Variables|Spawner|GetSpawnCooldown) true))
      (Variables|Spawner|SetSpawnTimerHandle _returnvalue))))

(event EventBeginPlay
  (CallFunction|StartSpawning))

(fn ConstructionScript)